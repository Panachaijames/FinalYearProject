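; BP_Gun is a gun item that a player picks up by interacting with it and that can be dropped again.
; A Dropped/Equipped state, set to Dropped on BeginPlay, switches the overlap sphere's collision and the skeletal mesh's physics and collision profile, resetting the mesh's relative transform when equipped.
; Interaction supplies a "Pick up" prompt attached to the mesh, passes the gun to the player's PickupGun, then equips it.
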(event EventBeginPlay
  (Private|SetGunState "NewEnumerator0"))

(event EventOnInteracted
  (params (Player :type Ue%204ASP%20Character%20Object%20Reference))
  (Default|PickupGun Player self)
  (Private|SetGunState "NewEnumerator1"))

(fn ConstructionScript
  (|CallParentFunction))

(fn GetInteractionText
  (return "Pick up"))

(fn GetInteractionTextAttach
  (return (Variables|Default|GetSkeletalMesh)))

(fn SetGunState
  (params (NewGunState :type EGunState%20Enum :default "NewEnumerator0"))
  (bind _skeletalmesh (Variables|Default|GetSkeletalMesh))
  (bind _skeletalmesh_2 (Variables|Default|GetSkeletalMesh))
  (bind _output_get (Variables|Private|SetGun%20State NewGunState))
  (switch Utilities|FlowControl|Switch|SwitchonEGunState _output_get
    (:NewEnumerator0
      (Collision|SetCollisionProfileName (Variables|Default|GetSphere) "OverlapAllDynamic" true :!class /Script/Engine.PrimitiveComponent)
      (Physics|SetSimulatePhysics _skeletalmesh_2 true)
      (Collision|SetCollisionProfileName _skeletalmesh_2 "DroppedGun" true :!class /Script/Engine.PrimitiveComponent))
    (:NewEnumerator1
      (Collision|SetCollisionProfileName (Variables|Default|GetSphere) "NoCollision" true :!class /Script/Engine.PrimitiveComponent)
      (Physics|SetSimulatePhysics _skeletalmesh false)
      (Collision|SetCollisionProfileName _skeletalmesh "NoCollision" true :!class /Script/Engine.PrimitiveComponent)
      (Transformation|ResetRelativeTransform (Variables|Default|GetSkeletalMesh)))))

(fn Drop
  (Private|SetGunState "NewEnumerator0"))